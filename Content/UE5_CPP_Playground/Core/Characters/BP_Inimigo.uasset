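; BP_Inimigo is an enemy actor that trades damage on contact, built around a BasicHealthSystem component.
; On BeginPlay it passes health, shield and stamina audio components to the health system and binds its destroyed event.
; When any overlap with its collider ends, it damages itself, and also damages the other actor if it is BP_ThirdPersonCharacter.
; On destruction it spawns a particle effect and plays a sound at its location.
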(event `self.ReceiveBeginPlay`
  (`BasicHealthSystem.SetLowAudioComponents` (`self.BasicHealthSystem`) (`self.HealthAudioComp`) (`self.ShieldAudioComp`) (`self.StaminaAudioComp`))
  (add `self.OnDestroyed` (delegate `Destroy`)))

(event `Destroy` :!signature `self.OnDestroyed`
  (params (DestroyedActor :type "Actor Object Reference"))
  (bind (_returnvalue_location _returnvalue_rotation _returnvalue_scale) (`KismetMathLibrary.BreakTransform` (`self.GetTransform`)))
  (`GameplayStatics.SpawnEmitterAtLocation` "/Engine/Tutorial/SubEditors/TutorialAssets/TutorialParticleSystem.TutorialParticleSystem" _returnvalue_location _returnvalue_rotation _returnvalue_scale)
  (`GameplayStatics.PlaySoundAtLocation` "/Engine/VREditor/Sounds/VR_teleport_Cue.VR_teleport_Cue" _returnvalue_location (struct) 1.0 1.0 0.0 null null null null))

(event `self.Collider.OnComponentEndOverlap`
  (params (OverlappedComponent :type "PrimitiveComponent Object Reference") (OtherActor :type "Actor Object Reference") (OtherComp :type "PrimitiveComponent Object Reference") (OtherBodyIndex :type Integer))
  (bind (_asbp_third_person_character _bsuccess) (cast `/Game/ThirdPerson/Blueprints/BP_ThirdPersonCharacter` OtherActor :!pure true))
  (`BasicHealthSystem.DealDamage` (`self.BasicHealthSystem`) 30.0)
  (if _bsuccess
    (`BasicHealthSystem.DealDamage` (`/Game/ThirdPerson/Blueprints/BP_ThirdPersonCharacter.BasicHealthSystem` _asbp_third_person_character) 25.0)))

(fn `UserConstructionScript`)